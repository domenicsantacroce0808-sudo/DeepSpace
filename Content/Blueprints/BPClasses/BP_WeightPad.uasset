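; Weight-sensitive pad that sinks as objects load it and reports its fill percentage to connected actors.
; SphereCollision overlaps add or remove each actor's component mass in a map, keeping a total clamped to the target weight.
; A change in percentage messages every connected actor and enables Tick.
; Tick interpolates the pad's height toward that percentage, then switches itself off once it matches.
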(event OnComponentBeginOverlap(SphereCollision)
  (params (OverlappedComponent :type Primitive%20Component%20Object%20Reference) (OtherActor :type Actor%20Object%20Reference) (OtherComp :type Primitive%20Component%20Object%20Reference) (OtherBodyIndex :type Integer) (bFromSweep :type Boolean) (SweepResult :type Hit%20Result%20Structure%20%28by%20ref%29))
  (CallFunction|ObjectIn/OutOfPad OtherActor OtherComp true)
  (CallFunction|UpdateStats))

(event OnComponentEndOverlap(SphereCollision)
  (params (OverlappedComponent :type Primitive%20Component%20Object%20Reference) (OtherActor :type Actor%20Object%20Reference) (OtherComp :type Primitive%20Component%20Object%20Reference) (OtherBodyIndex :type Integer))
  (CallFunction|ObjectIn/OutOfPad OtherActor OtherComp false)
  (CallFunction|UpdateStats))

(event EventBeginPlay)

(event Collision|EventActorBeginOverlap
  (params (OtherActor :type Actor%20Object%20Reference)))

(event EventTick
  (params (DeltaSeconds :type Float%20%28single-precision%29))
  (if (== (Variables|Default|GetPadOffSetAmount) (Variables|Default|GetCurrentWeightPercent))
    (Actor|Tick|SetActorTickEnabled false)
    (Development|PrintString "PadAticve")
    (else
      (Variables|Default|SetPadOffSetAmount (Math|Interpolation|FInterpTo (Variables|Default|GetPadOffSetAmount) (Variables|Default|GetCurrentWeightPercent) (Utilities|Time|GetWorldDeltaSeconds) 1e+01))
      (Variables|Default|SetPad%20Position (Math|Vector|MakeVector 0.0 0.0 (Math|Float|Lerp 1.6e+02 -5e+01 (Variables|Default|GetPadOffSetAmount))))
      (Transformation|SetRelativeLocation (Variables|Default|GetPad) (Variables|Default|GetPad%20Position) false false))))

(fn ConstructionScript)

(fn ObjectIn/OutOfPad
  (params (In%20Actor :type Actor%20Object%20Reference) (In%20Comp :type Primitive%20Component%20Object%20Reference) (Plus? :type Boolean))
  (bind _objectonpad_weight (Variables|Default|GetObjectOnPad+Weight))
  (bind _value (Utilities|Map|Find _objectonpad_weight In%20Actor))
  (if Plus?
    (Utilities|Map|Add (Variables|Default|GetObjectOnPad+Weight) In%20Actor (Physics|GetMass In%20Comp)))
  (if (Utilities|Map|IsEmpty (Variables|Default|GetObjectOnPad+Weight))
    (Variables|Default|SetCurrentWeightOnPad 0.0)
    (else
      (Variables|Default|SetCurrentWeightOnPad (Math|Float|Clamp(Float) (+ (Variables|Default|GetCurrentWeightOnPad) (select Plus? _value (* _value -1.0))) 0.0 (Variables|Default|GetTargetWeight)))))
  (if (not Plus?)
    (Utilities|Map|Remove (Variables|Default|GetObjectOnPad+Weight) In%20Actor)))

(fn UpdateStats
  (bind _currentweightonpad (Variables|Default|GetCurrentWeightOnPad))
  (bind _targetweight (Variables|Default|GetTargetWeight))
  (bind _returnvalue (/ _currentweightonpad _targetweight))
  (bind _returnvalue_2 (Math|Float|Clamp(Float) _returnvalue))
  (if (not (== (Variables|Default|GetCurrentWeightPercent) _returnvalue_2))
    (Variables|Default|SetCurrentWeightPercent _returnvalue_2)
    (Actor|Tick|SetActorTickEnabled true)
    (for _array_element (Variables|Default|GetConnectedActors)
      (Class|BPIWeightPad|CurrentWeightValues(Message) (Utilities|ResolveSoftReference _array_element) (Variables|Default|GetCurrentWeightPercent)))))