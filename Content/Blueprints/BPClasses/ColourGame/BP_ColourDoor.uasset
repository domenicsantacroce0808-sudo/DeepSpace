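; BP_ColourDoor is a door for the colour game that opens when all of its linked pads are activated.
; On BeginPlay it binds to each pad's activate and deactivate events, and every activation rechecks all pads, ignoring colour.
; A timeline lerps the door's relative location between closed and open.
; Deactivation only clears CurrentSequence; CloseDoor reverses the timeline but is not called within this Blueprint.
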(event Custom|OpenDoor
  ;[0.15 0.15 0.15 0.5] Open and Close Door Timeline
  (if (Variables|Default|GetIsDoorOpen)
    (Variables|Default|SetIsDoorOpen true)
    (bind _openalpha (Timeline|Timeline_Door Play)
      (:Update
        (bind _output_get (Variables|Default|SetNewLocation (Math|Vector|Lerp(Vector) (Variables|Default|GetClosedLocation) (Variables|Default|GetOpenLocation) _openalpha)))
        (Transformation|SetRelativeLocation (Variables|Default|GetDoor) _output_get false false)))
    (else
      (Timeline|Timeline_Door Play))))

(event Custom|CloseDoor
  ;[0.15 0.15 0.15 0.5] Open and Close Door Timeline
  (Variables|Default|SetIsDoorOpen false)
  (bind _openalpha (Timeline|Timeline_Door Reverse)
    (:Update
      (bind _output_get (Variables|Default|SetNewLocation (Math|Vector|Lerp(Vector) (Variables|Default|GetClosedLocation) (Variables|Default|GetOpenLocation) _openalpha)))
      (Transformation|SetRelativeLocation (Variables|Default|GetDoor) _output_get false false))))

(event Custom|PadActivate
  (params (PadRef :type BP%20Pressure%20Pad%20Object%20Reference) (SphereType :type E_SphereType%20Enum :default "NewEnumerator0"))
  ;[0.15 0.15 0.15 0.5] PadActivate/PadDeactivate Colour Door event
  (bind _success (CallFunction|CheckDoorCondition))
  (if _success
    (CallFunction|OpenDoor)))

(event Custom|PadDeactivate
  (params (PadRef :type BP%20Pressure%20Pad%20Object%20Reference))
  ;[0.15 0.15 0.15 0.5] PadActivate/PadDeactivate Colour Door event
  (Utilities|Array|Clear (Variables|Default|GetCurrentSequence)))

(event EventBeginPlay
  ;[0.15 0.15 0.15 0.5] PadActivate/PadDeactivate Colour Door event
  (for _array_element (Variables|Default|GetPads)
    (EventDispatchers|BindEventtoOnPadActivated _array_element (delegate Custom|PadActivate))
    (EventDispatchers|BindEventtoOnPadDeactivated _array_element (delegate Custom|PadDeactivate))))

(fn ConstructionScript)

(fn CheckDoorCondition
  (LocalVariables|SetbShould%20Door%20Open true)
  (bind _array_element (Utilities|Array|ForEachLoopwithBreak (Variables|Default|GetPads) :!label _label)
    (:LoopBody
      (if (not (Variables|/Game/Blueprints/BPClasses/ColourGame/BP_PressurePad.BP_PressurePad_C|GetIsActivated _array_element))
        (LocalVariables|SetbShould%20Door%20Open false)
        (goto _label Break)))
    (:Completed
      (return (LocalVariables|GetbShould%20Door%20Open)))))