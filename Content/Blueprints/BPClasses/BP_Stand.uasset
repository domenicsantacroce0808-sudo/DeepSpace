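; BP_Stand is a coloured stand for a Simon Says minigame that plays its own note and lights up.
; The construction script gives the capsule a dynamic material tinted with the stand's Colour, and BeginPlay assigns its Sound.
; An interact event from a BPI_Player actor calls PlayNote, which plays the sound and raises material Intensity briefly.
; A look-at event applies an overlay material to the capsule, using a retriggerable delay.
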(event Custom|PlayNote
  (Audio|Components|Audio|Play (Variables|Default|GetAudio) 0.0)
  (Rendering|Material|SetScalarParameterValue (Variables|Default|GetDynamic%20Material) "Intensity" 2.5 :!class /Script/Engine.MaterialInstanceDynamic)
  (Utilities|FlowControl|Delay 0.65)
  (Audio|Components|Audio|Stop (Variables|Default|GetAudio))
  (Rendering|Material|SetScalarParameterValue (Variables|Default|GetDynamic%20Material) "Intensity" 0.0 :!class /Script/Engine.MaterialInstanceDynamic))

(event EventEventInteractSImonSays
  (params (Actor :type Actor%20Object%20Reference))
  (if (Utilities|DoesObjectImplementInterface Actor "/Game/Blueprints/BPInterfaces/BPI_Player.BPI_Player_C")
    (if true
      (CallFunction|PlayNote))))

(event EventBeginPlay
  (Audio|Components|Audio|SetSound (Variables|Default|GetAudio) (Variables|Default|GetSound)))

(event EventOnLookat(simonSays)
  (params (Actor :type Actor%20Object%20Reference))
  (if true
    (Rendering|Material|SetOverlayMaterial (Variables|Default|GetCapsule) "/Game/Material/Colour(SImonSays)/M_Overlay.M_Overlay" :!class /Script/Engine.MeshComponent)
    (Utilities|FlowControl|RetriggerableDelay 0.11)
    (Rendering|Material|SetOverlayMaterial (Variables|Default|GetCapsule) "/Game/Material/Colour(SImonSays)/M_Overlay.M_Overlay" :!class /Script/Engine.MeshComponent)))

(fn ConstructionScript
  (bind _returnvalue (Rendering|Material|CreateDynamicMaterialInstance (Variables|Default|GetCapsule) 0 "/Game/Material/Colour(SImonSays)/M_Colour_Simon.M_Colour_Simon" "None" :!class /Script/Engine.PrimitiveComponent))
  (bind _output_get (Variables|Default|SetDynamic%20Material _returnvalue))
  (Rendering|Material|SetVectorParameterValue _output_get "Colour" (Variables|Default|GetColour) :!class /Script/Engine.MaterialInstanceDynamic))