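; BP_Sphere is a Blueprint that shows an interaction indicator, WInteract, while something overlaps its Trigger sphere.
; Overlap begin and end events on Trigger toggle the indicator's visibility, with no filter on the overlapping actor.
; Every Tick moves WInteract to the top of the sphere, offsetting it from the Trigger's location along its up vector by the scaled radius.
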(event OnComponentBeginOverlap(Trigger)
  (params (OverlappedComponent :type Primitive%20Component%20Object%20Reference) (OtherActor :type Actor%20Object%20Reference) (OtherComp :type Primitive%20Component%20Object%20Reference) (OtherBodyIndex :type Integer) (bFromSweep :type Boolean) (SweepResult :type Hit%20Result%20Structure%20%28by%20ref%29))
  (Rendering|SetVisibility (Variables|Default|GetW_Interact) true false))

(event OnComponentEndOverlap(Trigger)
  (params (OverlappedComponent :type Primitive%20Component%20Object%20Reference) (OtherActor :type Actor%20Object%20Reference) (OtherComp :type Primitive%20Component%20Object%20Reference) (OtherBodyIndex :type Integer))
  (Rendering|SetVisibility (Variables|Default|GetW_Interact) false false))

(event EventTick
  (params (DeltaSeconds :type Float%20%28single-precision%29))
  (Transformation|SetWorldLocation (Variables|Default|GetW_Interact) (+ (Transformation|GetWorldLocation (Variables|Default|GetTrigger)) (* (Math|Vector|GetUpVector (Variables|Default|GetTrigger)) (Components|Sphere|GetScaledSphereRadius (Variables|Default|GetTrigger)))) false false))

(fn ConstructionScript)