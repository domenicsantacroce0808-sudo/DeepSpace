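; BP_Pickup is a pickup item in the ColourGame that shows an "E" interaction widget while something overlaps its trigger zone.
; Trigger begin and end overlap events toggle the widget's visibility, with no check on which actor overlaps.
; Tick repositions the widget near a point one trigger radius along the Sphere's up vector, through a constant-speed interpolation with no target wired.
; The file contains no input or collection logic.
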(event OnComponentBeginOverlap(Trigger)
  (params (OverlappedComponent :type Primitive%20Component%20Object%20Reference) (OtherActor :type Actor%20Object%20Reference) (OtherComp :type Primitive%20Component%20Object%20Reference) (OtherBodyIndex :type Integer) (bFromSweep :type Boolean) (SweepResult :type Hit%20Result%20Structure%20%28by%20ref%29))
  ;[0.15 0.15 0.15 0.5] When Player Overlaps, widgets "E" Pick Me Up appears
  (Rendering|SetVisibility (Variables|Default|GetW_Interact) true false))

(event OnComponentEndOverlap(Trigger)
  (params (OverlappedComponent :type Primitive%20Component%20Object%20Reference) (OtherActor :type Actor%20Object%20Reference) (OtherComp :type Primitive%20Component%20Object%20Reference) (OtherBodyIndex :type Integer))
  ;[0.15 0.15 0.15 0.5] When Player Overlaps, widgets "E" Pick Me Up appears
  (Rendering|SetVisibility (Variables|Default|GetW_Interact) false false))

(event EventTick
  (params (DeltaSeconds :type Float%20%28single-precision%29))
  (bind _sphere (Variables|Default|GetSphere))
  ;[0.15 0.15 0.15 0.5] Controls floating pickup items and shows the ‘E’ interaction widget when the player enters the trigger zone
  (Transformation|SetWorldLocation (Variables|Default|GetW_Interact) (Math|Interpolation|VInterptoConstant (+ (Transformation|GetWorldLocation _sphere) (* (Math|Vector|GetUpVector _sphere) (Components|Sphere|GetScaledSphereRadius (Variables|Default|GetTrigger)))) "0, 0, 0" DeltaSeconds 5.0) false false))

(fn ConstructionScript)