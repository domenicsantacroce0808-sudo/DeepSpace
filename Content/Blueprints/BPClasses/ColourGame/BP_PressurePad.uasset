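; BP_PressurePad is a pressure pad for the colour game that detects BP_Pickup spheres in its trigger area.
; Any pickup entering sets IsActivated, but the OnPadActivated dispatcher fires only when its SphereType matches the pad's allowed type, passing the pad and type.
; Any pickup leaving clears the flag and fires OnPadDeactivated without a type check.
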(event OnComponentBeginOverlap(TriggerArea)
  (params (OverlappedComponent :type Primitive%20Component%20Object%20Reference) (OtherActor :type Actor%20Object%20Reference) (OtherComp :type Primitive%20Component%20Object%20Reference) (OtherBodyIndex :type Integer) (bFromSweep :type Boolean) (SweepResult :type Hit%20Result%20Structure%20%28by%20ref%29))
  ;[0.15 0.15 0.15 0.5] Activate Pressure Pad
  (bind _asbp_pickup (Utilities|Casting|CastToBP_Pickup OtherActor))
  (Variables|Default|SetIsActivated true)
  (if (Utilities|Enum|Equal(Enum) (Variables|/Game/Blueprints/BPClasses/ColourGame/BP_Pickup.BP_Pickup_C|GetSphereType _asbp_pickup) (Variables|Default|GetAllowedShpereType))
    (Default|CallOnPadActivated self (Variables|/Game/Blueprints/BPClasses/ColourGame/BP_Pickup.BP_Pickup_C|GetSphereType _asbp_pickup))))

(event OnComponentEndOverlap(TriggerArea)
  (params (OverlappedComponent :type Primitive%20Component%20Object%20Reference) (OtherActor :type Actor%20Object%20Reference) (OtherComp :type Primitive%20Component%20Object%20Reference) (OtherBodyIndex :type Integer))
  ;[0.15 0.15 0.15 0.5] Deactivate Pressure Pad
  (Utilities|Casting|CastToBP_Pickup OtherActor)
  (Variables|Default|SetIsActivated false)
  (if true
    (Default|CallOnPadDeactivated self)))

(fn ConstructionScript)