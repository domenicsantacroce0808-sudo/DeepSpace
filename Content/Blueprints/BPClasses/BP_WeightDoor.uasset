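; BP_WeightDoor is a door actor whose opening follows a weight percentage received through CurrentWeightValues.
; That event sets IsComplete at full weight and can snap partial values to closed via OnlyUpdateWhenComplete.
; Tick eases DoorOpenAmount toward the percentage with FInterpTo, slides the Door along relative X, and disables itself on arrival.
; CurrentWeightValues also disables tick, and nothing in these graphs re-enables it.
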(event EventTick
  (params (DeltaSeconds :type Float%20%28single-precision%29))
  (if (== (Variables|Default|GetDoorOpenAmount) (Variables|Default|GetWeight%20Percent))
    (Actor|Tick|SetActorTickEnabled false)
    (Development|PrintString "DoorActivate")
    (else
      (Variables|Default|SetDoorOpenAmount (Math|Interpolation|FInterpTo (Variables|Default|GetDoorOpenAmount) (Variables|Default|GetWeight%20Percent) (Utilities|Time|GetWorldDeltaSeconds) 1e+01))
      (Variables|Default|SetDoorPosition (Math|Vector|MakeVector (Math|Float|Lerp 145.0 3e+01 (Variables|Default|GetDoorOpenAmount)) 0.0 0.0))
      (Transformation|SetRelativeLocation (Variables|Default|GetDoor) (Variables|Default|GetDoorPosition) false false))))

(event EventCurrentWeightValues
  (params (WeightPercent :type Float%20%28double-precision%29))
  (bind _returnvalue (== WeightPercent 1.0))
  (if (Variables|Default|GetOnlyUpdateWhenComplete)
    (Variables|Default|SetWeight%20Percent (Math|Conversions|ToFloat(Boolean) _returnvalue))
    (else
      (Variables|Default|SetWeight%20Percent WeightPercent)))
  (Variables|Default|SetIsComplete _returnvalue)
  (Actor|Tick|SetActorTickEnabled false)
  (Development|PrintString "WeightActive"))

(fn ConstructionScript)