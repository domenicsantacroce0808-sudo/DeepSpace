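; BP_Stand is one coloured note stand in a Simon Says minigame, with its own index, colour and sound.
; When a player interacts during their turn, it reports its index to the main Simon actor, and when looked at then it shows a brief retriggerable overlay highlight.
; PlayNote and PlayError briefly play audio and light a dynamic material, with the error swapping in red and an error sound before restoring both.
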(event Custom|PlayError
  (Audio|Components|Audio|SetSound (Variables|Default|GetAudio) "/Game/Sounds/AudioSound(Simon)/soundshelfstudio-ui-error-pop-515668.soundshelfstudio-ui-error-pop-515668")
  (Audio|Components|Audio|Play (Variables|Default|GetAudio) 0.0)
  (Rendering|Material|SetVectorParameterValue (Variables|Default|GetDynamic%20Material) "Colour" "(R=1.000000,G=0.000000,B=0.007453,A=1.000000)" :!class /Script/Engine.MaterialInstanceDynamic)
  (Rendering|Material|SetScalarParameterValue (Variables|Default|GetDynamic%20Material) "Intensity" 2.5 :!class /Script/Engine.MaterialInstanceDynamic)
  (Utilities|FlowControl|Delay 0.65)
  (Audio|Components|Audio|Stop (Variables|Default|GetAudio))
  (Rendering|Material|SetScalarParameterValue (Variables|Default|GetDynamic%20Material) "Intensity" 0.0 :!class /Script/Engine.MaterialInstanceDynamic)
  (Rendering|Material|SetVectorParameterValue (Variables|Default|GetDynamic%20Material) "Colour" (Variables|Default|GetColour) :!class /Script/Engine.MaterialInstanceDynamic)
  (Audio|Components|Audio|SetSound (Variables|Default|GetAudio) (Variables|Default|GetSound)))

(event Custom|PlayNote
  (Audio|Components|Audio|Play (Variables|Default|GetAudio) 0.0)
  (Rendering|Material|SetScalarParameterValue (Variables|Default|GetDynamic%20Material) "Intensity" 2.5 :!class /Script/Engine.MaterialInstanceDynamic)
  (Utilities|FlowControl|Delay 0.65)
  (Audio|Components|Audio|Stop (Variables|Default|GetAudio))
  (Rendering|Material|SetScalarParameterValue (Variables|Default|GetDynamic%20Material) "Intensity" 0.0 :!class /Script/Engine.MaterialInstanceDynamic))

(event EventEventInteractSImonSays
  (params (Actor :type Actor%20Object%20Reference))
  (if (Utilities|DoesObjectImplementInterface Actor "/Game/Blueprints/BPInterfaces/BPI_Player.BPI_Player_C")
    (bind _simonmain_reference (Variables|Default|GetSimonMain_Reference)
      (:then
        (if (Variables|/Game/Blueprints/BPClasses/SimonSaysGame/BP_SimonMain.BP_SimonMain_C|GetIsPlayersTurn _simonmain_reference)
          (Default|PlayerPlayedNote (Variables|Default|GetSimonMain_Reference) (Variables|Default|GetIndex))))
      (:else))))

(event EventBeginPlay
  (Audio|Components|Audio|SetSound (Variables|Default|GetAudio) (Variables|Default|GetSound)))

(event EventOnLookat(simonSays)
  (params (Actor :type Actor%20Object%20Reference))
  (bind _simonmain_reference (Variables|Default|GetSimonMain_Reference)
    (:then
      (if (Variables|/Game/Blueprints/BPClasses/SimonSaysGame/BP_SimonMain.BP_SimonMain_C|GetIsPlayersTurn _simonmain_reference)
        (Rendering|Material|SetOverlayMaterial (Variables|Default|GetCapsule) "/Game/Material/Colour(SImonSays)/M_Overlay.M_Overlay" :!class /Script/Engine.MeshComponent)
        (Utilities|FlowControl|RetriggerableDelay 0.11)
        (Rendering|Material|SetOverlayMaterial (Variables|Default|GetCapsule) 0 :!class /Script/Engine.MeshComponent)))
    (:else)))

(fn ConstructionScript
  (bind _returnvalue (Rendering|Material|CreateDynamicMaterialInstance (Variables|Default|GetCapsule) 0 "/Game/Material/Colour(SImonSays)/M_Colour_Simon.M_Colour_Simon" "None" :!class /Script/Engine.PrimitiveComponent))
  (bind _output_get (Variables|Default|SetDynamic%20Material _returnvalue))
  (Rendering|Material|SetVectorParameterValue _output_get "Colour" (Variables|Default|GetColour) :!class /Script/Engine.MaterialInstanceDynamic))